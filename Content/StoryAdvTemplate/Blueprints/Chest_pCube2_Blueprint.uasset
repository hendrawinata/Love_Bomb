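; Interactable chest for a story adventure template that opens and closes its lid when the game controller allows it.
; Interaction checks CanOpenChest on BP_GameController, then toggles IsOpen and plays the OpenChest timeline forward or in reverse to rotate the Tutup component on roll.
; Sounds play at the player for both toggle and refusal.
; The controller's HoldTrace is held during interaction, including a short delay after each toggle.
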(event `self.ReceiveBeginPlay`
  ;[1 1 1] Set Character Instance
  (bind _outactors (`GameplayStatics.GetAllActorsOfClass` "/Game/StoryAdvTemplate/Blueprints/BP_GameController.BP_GameController_C"))
  (set `self.Game Controller Instance` (`|GetArrayItem` _outactors)))

(event `Open Chest`
  ;[1 1 1] Open Chest
  (bind (_direction _openchestfloat) (`Timeline|OpenChest` :!via `PlayFromStart` :!label _label)
    (:`Update`
      (`SceneComponent.K2_SetRelativeRotation` (`self.Tutup`) (`KismetMathLibrary.MakeRotator` _openchestfloat) false false))))

(event `CloseChest`
  (goto _label :!via `ReverseFromEnd`))

(event `self.Interaction`
  (bind _returnvalue (`self.K2_GetActorLocation` (`GameplayStatics.GetPlayerCharacter` 0)))
  ;[1 1 1] Check Open Chest
  (if (not (`self.isMoving?`))
    (set `/Game/StoryAdvTemplate/Blueprints/BP_GameController.HoldTrace` true (`self.Game Controller Instance`))
    (if (`/Game/StoryAdvTemplate/Blueprints/BP_GameController.Can Open Chest ?` (`self.Game Controller Instance`))
      (if (`self.isOpen?`)
        (`self.CloseChest`)
        (set `self.isOpen?` false)
        (`GameplayStatics.PlaySoundAtLocation` "/Game/StoryAdvTemplate/Sound/Waves/Chest_Cue.Chest_Cue" _returnvalue (struct) 1.0 1.0 0.0 null null null)
        (else
          (`self.Open Chest`)
          (set `self.isOpen?` true)
          (`GameplayStatics.PlaySoundAtLocation` "/Game/StoryAdvTemplate/Sound/Waves/Chest_Cue.Chest_Cue" _returnvalue (struct) 1.0 1.0 0.0 null null null)))
      (`KismetSystemLibrary.Delay` 1.0)
      (else
        (`GameplayStatics.PlaySoundAtLocation` "/Game/StoryAdvTemplate/Sound/Cues/SC_CloseDoor.SC_CloseDoor" (`SceneComponent.K2_GetComponentLocation` (`Character.Mesh` (`GameplayStatics.GetPlayerCharacter` 0))) (struct) 1.0 1.0 0.0 null null null)))
    (set `self.isMoving?` false)
    (set `/Game/StoryAdvTemplate/Blueprints/BP_GameController.HoldTrace` false (`self.Game Controller Instance`))))

(fn `UserConstructionScript`)